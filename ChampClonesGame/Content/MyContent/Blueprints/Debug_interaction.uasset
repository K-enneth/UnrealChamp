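; Debug interactable Blueprint that opens and closes a pair of doors, DoorL and DoorR, when DefaultInteract fires.
; Each door has a FlipFlop that alternately plays and reverses its timeline, sliding the door along relative X.
; The left timeline value is scaled into Angle, which drives DoorL's offset and blocks interaction until it nears either end of travel.
; DoorR uses its timeline value unscaled.
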(event `/Game/MyContent/Blueprints/Interactions.DefaultInteract`
  (bind _angle (`self.Angle`))
  (if (or (< _angle 1.0) (> _angle 119.0))
    (`|ExecutionSequence`
      (:`then_0`
        (`/Engine/EditorBlueprintResources/StandardMacros.FlipFlop`
          (:`A`
            (bind (_direction _value) (`Timeline|DoorLM` :!label _label)
              (:`Update`
                (bind _output_get (set `self.Angle` (* _value 120.0)))
                (`SceneComponent.K2_SetRelativeLocation` (`self.DoorL`) (`KismetMathLibrary.MakeVector` _output_get) false false))))
          (:`B`
            (goto _label :!via `Reverse`))))
      (:`then_1`
        (`/Engine/EditorBlueprintResources/StandardMacros.FlipFlop`
          (:`A`
            (bind (_direction_2 _value_2) (`Timeline|DoorRM` :!label _label_2)
              (:`Update`
                (`SceneComponent.K2_SetRelativeLocation` (`self.DoorR`) (`KismetMathLibrary.MakeVector` _value_2) false false))))
          (:`B`
            (goto _label_2 :!via `Reverse`)))))))

(fn `UserConstructionScript`)