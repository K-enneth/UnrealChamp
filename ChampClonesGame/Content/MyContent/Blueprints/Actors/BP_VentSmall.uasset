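; BP_VentSmall is a small vent actor that teleports the player to a stored location on interaction.
; SmallInteract fades the camera out, waits for the fade to finish, moves the player character to NewLocation, then stops the fade.
; Any actor overlap creates a SmallCWidger widget on screen, and ending the overlap removes all widgets rather than just that one.
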(event `/Game/MyContent/Blueprints/Interactions.SmallInteract`
  (bind _returnvalue (`GameplayStatics.GetPlayerCameraManager` 0))
  (`PlayerCameraManager.StartCameraFade` :`self` _returnvalue :`ToAlpha` 1.0 :`Duration` 0.5 :`bHoldWhenFinished` true)
  (`KismetSystemLibrary.Delay` 0.5)
  (`self.K2_SetActorLocation` (`GameplayStatics.GetPlayerCharacter` 0) (`self.NewLocation`) false false)
  (`PlayerCameraManager.StopCameraFade` _returnvalue))

(event `self.ReceiveActorBeginOverlap`
  (params (OtherActor :type "Actor Object Reference"))
  (bind _returnvalue (`|CreateWidget` "/Game/MyContent/Widgets/SmallCWidger.SmallCWidger_C"))
  (`UserWidget.AddToViewport` _returnvalue 0))

(event `self.ReceiveActorEndOverlap`
  (params (OtherActor :type "Actor Object Reference"))
  (`WidgetLayoutLibrary.RemoveAllWidgets`))

(fn `UserConstructionScript`)