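; BP_TestTube is an interactable test tube actor that releases a big clone and unlocks a character for the player.
; Overlap events enable input and open a gate, so the E key only works while something is inside its bounds.
; If the BP_CharacterSwitch controller's CanOpenTube is set, a DoOnce spawns BP_BigClone at BigSpawn and calls UnlockChar on that controller.
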(event `Key|E`
  (params (Key :type "Key Structure"))
  (:`Pressed`
    (`/Engine/EditorBlueprintResources/StandardMacros.Gate` true :!label _label
      (:`Exit`
        (bind _asbp_character_switch (cast `/Game/MyContent/Blueprints/Characters/BP_CharacterSwitch` (`GameplayStatics.GetPlayerController` 0)))
        (if (`/Game/MyContent/Blueprints/Characters/BP_CharacterSwitch.CanOpenTube` _asbp_character_switch)
          (`/Engine/EditorBlueprintResources/StandardMacros.DoOnce` false
            (:`Completed`
              (`|SpawnActorFromClass` "/Game/MyContent/Blueprints/Characters/BP_BigClone.BP_BigClone_C" (`KismetMathLibrary.MakeTransform` (`self.Big spawn`)) "Undefined" "MultiplyWithRoot" null null)
              (bind _asbp_character_switch_2 (cast `/Game/MyContent/Blueprints/Characters/BP_CharacterSwitch` (`GameplayStatics.GetPlayerController` 0)))
              (`/Game/MyContent/Blueprints/Characters/BP_CharacterSwitch.UnlockChar` _asbp_character_switch_2))))))))

(event `self.ReceiveActorBeginOverlap`
  (params (OtherActor :type "Actor Object Reference"))
  (`self.EnableInput` (`GameplayStatics.GetPlayerController` 0))
  (goto _label :!via `Open`))

(event `self.ReceiveActorEndOverlap`
  (params (OtherActor :type "Actor Object Reference"))
  (`self.DisableInput` (`GameplayStatics.GetPlayerController` 0))
  (goto _label :!via `Close`))

(fn `UserConstructionScript`)