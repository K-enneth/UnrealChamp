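; BP_TubeKey is a key pickup actor that lets the player open a tube.
; An overlap shows its widget component, and ending the overlap hides it.
; DefaultInteract shows an ItemPicked message with the item name, hides the actor, and removes all widgets after a short delay.
; It then casts the player controller to BP_CharacterSwitch, sets CanOpenTube and destroys itself.
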(event `/Game/MyContent/Blueprints/Interactions.DefaultInteract`
  (bind _returnvalue (`|CreateWidget` "/Game/MyContent/Widgets/ItemPicked.ItemPicked_C"))
  (message `/Game/MyContent/Blueprints/PickUps.Picked` _returnvalue (`self.Name`))
  (`UserWidget.AddToViewport` _returnvalue 0)
  (`self.SetActorHiddenInGame` true)
  (`KismetSystemLibrary.Delay` 2.0)
  (`WidgetLayoutLibrary.RemoveAllWidgets`)
  (bind _asbp_character_switch (cast `/Game/MyContent/Blueprints/Characters/BP_CharacterSwitch` (`GameplayStatics.GetPlayerController` 0)))
  (set `/Game/MyContent/Blueprints/Characters/BP_CharacterSwitch.CanOpenTube` true _asbp_character_switch)
  (`self.K2_DestroyActor`))

(event `self.ReceiveActorBeginOverlap`
  (params (OtherActor :type "Actor Object Reference"))
  (`SceneComponent.SetHiddenInGame` (`self.Widget`) false false))

(event `self.ReceiveActorEndOverlap`
  (params (OtherActor :type "Actor Object Reference"))
  (`SceneComponent.SetHiddenInGame` (`self.Widget`) true false))

(fn `UserConstructionScript`)