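; BP_CharacterSwitch lets the player cycle control between the BP_ThirdPersonCharacter instances in the level.
; BeginPlay caches all those characters in an array and records the current player character.
; Pressing Enter calls ChangeChar only while the current character's last update velocity is zero.
; ChangeChar selects the next array entry, wrapping to the first past the end, and possesses it.
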(event `self.ReceiveBeginPlay`
  (bind _outactors (`GameplayStatics.GetAllActorsOfClass` "/Game/ThirdPerson/Blueprints/BP_ThirdPersonCharacter.BP_ThirdPersonCharacter_C"))
  (set `self.Characters` _outactors)
  (bind _asbp_third_person_character (cast `/Game/ThirdPerson/Blueprints/BP_ThirdPersonCharacter` (`GameplayStatics.GetPlayerCharacter` 0)))
  (set `self.CurrentChar` _asbp_third_person_character))

(event `Key|Enter`
  (params (Key :type "Key Structure"))
  (:`Pressed`
    (if (not (> (`KismetMathLibrary.VSize` (`CharacterMovementComponent.GetLastUpdateVelocity` (`Character.CharacterMovement` (`self.CurrentChar`)))) 0.0))
      (`self.ChangeChar`))))

(fn `ChangeChar`
  (locals (LocalIndex :type Integer))
  (bind _returnvalue (`KismetArrayLibrary.Array_Find` (`self.Characters`) (`self.CurrentChar`)))
  (bind _returnvalue_2 (+ _returnvalue 1))
  (set `local.LocalIndex` _returnvalue)
  (bind _output_get (set `local.LocalIndex` (`KismetMathLibrary.SelectInt` _returnvalue_2 0 (`KismetArrayLibrary.Array_IsValidIndex` (`self.Characters`) _returnvalue_2))))
  (bind _output_get_2 (set `self.CurrentChar` (`|GetArrayItem` (`self.Characters`) _output_get)))
  (`self.Possess` _output_get_2))

(fn `UserConstructionScript`)